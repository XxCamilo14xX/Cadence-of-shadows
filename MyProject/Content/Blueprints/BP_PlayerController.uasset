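; Player controller that routes Enhanced Input actions to the player pawn.
; On BeginPlay it caches the controlled pawn's interaction component, then maps the interaction action's press phases to begin, ongoing hold and end calls on it.
; Ending or canceling an interaction also unbinds all ongoing-press listeners.
; Move, dash and attack inputs are forwarded to player pawn 0 as message calls.
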(event Input|EnhancedActionEvents|EnhancedInputActionIA_Interaction
  (params (ActionValue :type Boolean) (ElapsedSeconds :type Float%20%28double-precision%29) (TriggeredSeconds :type Float%20%28double-precision%29) (InputAction :type Input%20Action%20Object%20Reference :default "/Game/Blueprints/Input/Actions/IA_Interaction.IA_Interaction"))
  (bind _playerinteraction (Variables|Default|GetPlayerInteraction))
  ;[0.15 0.15 0.15 0.5] Interactions
  (:Started
    (Default|InteractionBegin _playerinteraction))
  (:Ongoing
    (Default|CallOnInteractPressOngoing _playerinteraction ElapsedSeconds))
  (:Canceled
    (EventDispatchers|UnbindallEventsfromOnInteractPressOngoing _playerinteraction :!label _label)
    (Default|CallOnInteractEnded _playerinteraction))
  (:Completed
    (goto _label)))

(event Input|EnhancedActionEvents|EnhancedInputActionIA_Move
  (params (ActionValue :type Vector%202D%20Structure) (ElapsedSeconds :type Float%20%28double-precision%29) (TriggeredSeconds :type Float%20%28double-precision%29) (InputAction :type Input%20Action%20Object%20Reference :default "/Game/Blueprints/Input/Actions/IA_Move.IA_Move"))
  ;[0.05098 0.05098 0.05098] Movement
  (Class|BPIMoveSet|Move(Message) (Game|Player|GetPlayerPawn 0) ActionValue))

(event Input|EnhancedActionEvents|EnhancedInputActionIA_dash
  (params (ActionValue :type Boolean) (ElapsedSeconds :type Float%20%28double-precision%29) (TriggeredSeconds :type Float%20%28double-precision%29) (InputAction :type Input%20Action%20Object%20Reference :default "/Game/Blueprints/Input/Actions/IA_dash.IA_dash"))
  ;[0.05098 0.05098 0.05098] Dash Input
  (Class|BPIMoveSet|Dash(Message) (Game|Player|GetPlayerPawn 0)))

(event Input|EnhancedActionEvents|EnhancedInputActionIA_Attack
  (params (ActionValue :type Boolean) (ElapsedSeconds :type Float%20%28double-precision%29) (TriggeredSeconds :type Float%20%28double-precision%29) (InputAction :type Input%20Action%20Object%20Reference :default "/Game/Blueprints/Input/Actions/IA_Attack.IA_Attack"))
  ;[0.15 0.15 0.15 0.5] Attack
  (Class|BPIMoveSet|Melee(Message) (Game|Player|GetPlayerPawn 0)))

(event EventBeginPlay
  (Variables|Default|SetPlayerInteraction (Actor|GetComponentbyClass (Pawn|GetControlledPawn) "/Game/Blueprints/Components/BPC_Interaction_Systemm.BPC_Interaction_Systemm_C")))

(fn ConstructionScript)