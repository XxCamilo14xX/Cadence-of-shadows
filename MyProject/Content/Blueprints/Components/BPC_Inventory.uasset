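; BPC_Inventory is an inventory component that holds an item array and manages the inventory UI.
; On BeginPlay it creates a WB_inventory widget, sizes Items to twelve slots and passes itself to the widget's LoadInventory.
; The IA_Inventory input toggles the widget by adding it to or removing it from the viewport.
; AddItem is a stub that always returns false.
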(event Input|EnhancedActionEvents|EnhancedInputActionIA_Inventory
  (params (ActionValue :type Boolean) (ElapsedSeconds :type Float%20%28double-precision%29) (TriggeredSeconds :type Float%20%28double-precision%29) (InputAction :type Input%20Action%20Object%20Reference :default "/Game/Blueprints/Input/Actions/IA_Inventory.IA_Inventory"))
  (bind _inventorywidget (Variables|Default|GetInventorywidget))
  (:Started
    (if (Widget|IsVisible (Variables|Default|GetInventorywidget))
      (Widget|RemovefromParent _inventorywidget)
      (else
        (UserInterface|Viewport|AddtoViewport _inventorywidget 0)))))

(event EventBeginPlay
  (bind _returnvalue (UserInterface|CreateWidget "/Game/Blueprints/Inventory/Widget/WB_inventory.WB_inventory_C"))
  (Variables|Default|SetInventorywidget _returnvalue)
  (Utilities|Array|Resize (Variables|Default|GetItems) 12)
  (Default|LoadInventory (Variables|Default|GetInventorywidget) self))

(fn AddItem
  (params (Item :type S%20Item%20Struct%20Structure))
  (return false))