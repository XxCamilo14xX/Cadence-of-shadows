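; Inventory component that holds an Items array and shows or hides the inventory screen.
; On BeginPlay it creates and stores a WB_inventory widget and resizes Items to a fixed slot count.
; Pressing Tab toggles that same widget on and off the viewport based on its visibility.
; The graph has no logic for adding items or passing them to the widget.
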(event EventBeginPlay
  (bind _returnvalue (UserInterface|CreateWidget "/Game/Blueprints/Inventory/Widget/WB_inventory.WB_inventory_C"))
  (Variables|Default|SetInventorywidget _returnvalue)
  (Utilities|Array|Resize (Variables|Default|GetItems) 10))

(event EventTick
  (params (DeltaSeconds :type Float%20%28single-precision%29)))

(event Input|KeyboardEvents|Tab
  (params (Key :type Key%20Structure :default "None"))
  (bind _inventorywidget (Variables|Default|GetInventorywidget))
  (:Pressed
    (if (Widget|IsVisible (Variables|Default|GetInventorywidget))
      (Widget|RemovefromParent _inventorywidget)
      (else
        (UserInterface|Viewport|AddtoViewport _inventorywidget 0)))))