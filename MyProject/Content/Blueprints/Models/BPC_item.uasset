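; Pickup item actor that an interactor can collect through an interaction interface.
; The construction script applies the mesh from its Item data and enables physics simulation.
; On interaction it sends the interactor an item hardcoded as "Knife", rather than its own Item data, and destroys itself if the add succeeds.
; The interaction getters return fixed defaults: zero cost, hold time and location, plus the first interaction type.
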(event EventInteracti
  (params (Interactor :type Actor%20Object%20Reference))
  (bind _wasaded (Class|BPIInventory|AddItem(Message) Interactor (Utilities|Struct|MakeS_ItemStruct "Knife" "NewEnumerator0" false 0 0 0)))
  (if _wasaded
    (Actor|DestroyActor)))

(fn ConstructionScript
  (bind _staticmesh (Variables|Default|GetStaticMesh))
  (Components|StaticMesh|SetStaticMesh _staticmesh (.Mesh (Utilities|Struct|BreakS_ItemStruct (Variables|Default|GetItem))))
  (Physics|SetSimulatePhysics _staticmesh true))

(fn GetApCount
  (return 0))

(fn GetHoldDuration
  (return 0.0))

(fn GetInteractionLocation
  (return "0, 0, 0"))

(fn GetTypeInteraction
  (return "NewEnumerator0"))