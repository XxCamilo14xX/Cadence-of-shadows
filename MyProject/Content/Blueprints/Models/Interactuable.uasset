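; Interactuable is an interactable actor that works as a one-use healing pickup.
; On the Interacti event it sends a fixed Heal interface message to the interactor, then destroys itself.
; The other interaction, health and damage functions are stubs returning zero or default values, so it has no health of its own and ignores damage.
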(event EventInteracti
  (params (Interactor :type Actor%20Object%20Reference))
  (Class|BPIDamagable|Heal(Message) Interactor 2e+01)
  (Actor|DestroyActor))

(fn ConstructionScript)

(fn GetApCount
  (return 0))

(fn GetCurrentHealth
  (return 0.0))

(fn GetHoldDuration
  (return 0.0))

(fn GetInteractionLocation
  (return "0, 0, 0"))

(fn GetMaxHealth
  (return 0.0))

(fn GetTypeInteraction
  (return "NewEnumerator0"))

(fn Heal
  (params (Amount :type Float%20%28double-precision%29))
  (return 0.0))

(fn TakeDamage
  (params (DamgeInfo :type S%20Damage%20Info%20Structure))
  (return false))