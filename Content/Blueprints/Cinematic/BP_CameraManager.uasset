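; BP_CameraManager switches the local player's view between registered cinematic cameras and back to the player pawn.
; On BeginPlay it passes itself to the game instance through SetCameraManagerMessage.
; Cameras register by ID into a map, and SwitchToCamera blends the view to a found entry over a given time.
; ReturnToPlayer blends back to the pawn and resets ignored look and move input.
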(event EventBeginPlay
  (Class|BPICameraManager|SetCameraManager(Message) (Game|GetGameInstance) self))

(fn ConstructionScript)

(fn ReturntoPlayer
  (params (BlendTime :type Float%20%28double-precision%29))
  (bind _returnvalue (Game|GetPlayerController 0))
  (Game|Player|SetViewTargetwithBlend _returnvalue (Game|Player|GetPlayerPawn 0) BlendTime "VTBlend_Linear" 0.0 false)
  (Input|ResetIgnoreLookInput _returnvalue)
  (Input|ResetIgnoreMoveInput _returnvalue))

(fn RegisterCamera
  (params (CameraID :type Name) (Camera :type Actor%20Object%20Reference))
  (Utilities|Map|Add (Variables|Default|GetCameras) CameraID Camera))

(fn SwitchtoCamera
  (params (CameraID :type Name) (BlendTime :type Float%20%28double-precision%29))
  (bind _cameras (Variables|Default|GetCameras))
  (bind (_value _returnvalue) (Utilities|Map|Find _cameras CameraID))
  (if _returnvalue
    (Game|Player|SetViewTargetwithBlend (Game|GetPlayerController 0) _value BlendTime "VTBlend_Linear" 0.0 false)))