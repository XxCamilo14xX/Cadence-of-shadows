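; Camera manager that registers cinematic cameras by ID and handles blended view changes for the first player controller.
; On BeginPlay it passes itself to the Game Instance through SetCameraManagerMessage.
; RegisterCamera fills the Cameras map, and ReturnToPlayer blends the view back to the player pawn.
; SwitchToCamera starts a blend when the ID is found, but shows no new view target passed to it.
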(event EventBeginPlay
  (Class|BPICameraManager|SetCameraManager(Message) (Game|GetGameInstance) self))

(fn ConstructionScript)

(fn ReturntoPlayer
  (params (BlendTime :type Float%20%28double-precision%29))
  (Game|Player|SetViewTargetwithBlend (Game|GetPlayerController 0) (Game|Player|GetPlayerPawn 0) BlendTime "VTBlend_Linear" 0.0 false))

(fn RegisterCamera
  (params (CameraID :type Name) (Camera :type Actor%20Object%20Reference))
  (Utilities|Map|Add (Variables|Default|GetCameras) CameraID Camera))

(fn SwitchtoCamera
  (params (CameraID :type Name) (BlendTime :type Float%20%28double-precision%29))
  (if (.ReturnValue (Utilities|Map|Find (Variables|Default|GetCameras) CameraID))
    (Game|Player|SetViewTargetwithBlend (Game|GetPlayerController 0) 0 BlendTime "VTBlend_Linear" 0.0 false)))