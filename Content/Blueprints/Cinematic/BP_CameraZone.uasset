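; Camera zone that switches the view between its own camera and the player's.
; Box overlap reports its CameraID to the game instance, whose camera event triggers an immediate, timed or exit-based switch or return via game instance messages.
; Tick optionally follows the player at an offset, looks at them, or interpolates along a spline rail.
; Lock input modes call SetIgnoreLookInput/SetIgnoreMoveInput with false, so they never actually block input.
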(event OnComponentEndOverlap(Box)
  (params (OverlappedComponent :type Primitive%20Component%20Object%20Reference) (OtherActor :type Actor%20Object%20Reference) (OtherComp :type Primitive%20Component%20Object%20Reference) (OtherBodyIndex :type Integer))
  (if (== OtherActor (Game|Player|GetPlayerPawn 0))
    (switch Utilities|FlowControl|Switch|SwitchonE_CameraBehavior (Variables|Camera|GetCameraBehavior)
      (:NewEnumerator0
        (|ExitEvent)))))

(event OnComponentBeginOverlap(Box)
  (params (OverlappedComponent :type Primitive%20Component%20Object%20Reference) (OtherActor :type Actor%20Object%20Reference) (OtherComp :type Primitive%20Component%20Object%20Reference) (OtherBodyIndex :type Integer) (bFromSweep :type Boolean) (SweepResult :type Hit%20Result%20Structure%20%28by%20ref%29))
  (if (== OtherActor (Game|Player|GetPlayerPawn 0))
    (Class|BPICameraManager|ReportCameraEvent(Message) (Game|GetGameInstance) (Variables|Camera|GetCameraID))))

(event Custom|CameraEvent
  (params (CameraID :type Name))
  (bind _returnvalue (Game|GetPlayerController 0))
  (if (== CameraID (Variables|Camera|GetCameraID))
    (Utilities|FlowControl|Sequence
      (:then_0
        (switch Utilities|FlowControl|Switch|SwitchonE_CameraBehavior (Variables|Camera|GetCameraBehavior)
          (:NewEnumerator0
            (|RegularEvent :!label _label))
          (:NewEnumerator1
            (goto _label))
          (:NewEnumerator2
            (|ReturnEvent))
          (:NewEnumerator3
            (|TimedReturnEvent))
          (:NewEnumerator4
            (goto _label))))
      (:then_1
        (switch Utilities|FlowControl|Switch|SwitchonE_CameraInputMode (Variables|Camera|GetCameraInputMode)
          (:NewEnumerator1
            _)
          (:NewEnumerator2
            (Input|SetIgnoreMoveInput _returnvalue false)))
        (Input|SetIgnoreLookInput _returnvalue false)))))

(event EventBeginPlay
  (Utilities|FlowControl|Delay 1.0)
  (EventDispatchers|BindEventtoOnCameraEvent (CallFunction|GetMyGameInstance) (delegate Custom|CameraEvent))
  (Class|BPICameraManager|RegisterCamera(Message) (Game|GetGameInstance) (Variables|Camera|GetCameraID) self)
  (Variables|Default|SetOffset (Variables|/Script/Engine.SceneComponent|GetRelativeLocation (Variables|Default|GetCamera))))

(event EventTick
  (params (DeltaSeconds :type Float%20%28single-precision%29))
  (bind _camera (Variables|Default|GetCamera))
  (Utilities|FlowControl|Sequence
    (:then_0
      (switch Utilities|FlowControl|Switch|SwitchonE_CameraFollowMode (Variables|Camera|GetCameraFollowMode)
        (:NewEnumerator1
          (|FollowPlayerEvent))
        (:NewEnumerator2
          (|LookAtPlayerEvent))))
    (:then_1
      (switch Utilities|FlowControl|Switch|SwitchonE_CameraBehavior (Variables|Camera|GetCameraBehavior)
        (:NewEnumerator4
          (Transformation|SetWorldLocation _camera (Math|Interpolation|VInterpTo (Transformation|GetWorldLocation _camera) (Spline|FindLocationClosesttoWorldLocation (Variables|Default|GetSpline) (Transformation|GetActorLocation (Game|Player|GetPlayerPawn 0)) "World") (Utilities|Time|GetWorldDeltaSeconds) (Variables|Camera|GetInterpSpeed)) false false))))))

(fn ConstructionScript)

(event Custom|Return
  (Class|BPICameraManager|ReturntoPlayer(Message) (Game|GetGameInstance) (Variables|Camera|GetEndBlendTime)))