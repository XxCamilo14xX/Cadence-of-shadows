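; Teleport trigger actor that moves the player pawn to a set destination behind a camera fade.
; When the player pawn overlaps the box, the camera fades out, the pawn teleports with zeroed rotation, and the camera fades back in.
; After the teleport, an IsInteriorMessage call passes the IsInterior flag to the pawn.
; A DoOnce gate blocks retriggering during the sequence and resets after a further delay.
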(event OnComponentBeginOverlap(Box)
  (params (OverlappedComponent :type Primitive%20Component%20Object%20Reference) (OtherActor :type Actor%20Object%20Reference) (OtherComp :type Primitive%20Component%20Object%20Reference) (OtherBodyIndex :type Integer) (bFromSweep :type Boolean) (SweepResult :type Hit%20Result%20Structure%20%28by%20ref%29))
  (bind _returnvalue (Game|GetPlayerCameraManager 0))
  (if (== OtherActor (Game|Player|GetPlayerPawn 0))
    (Utilities|FlowControl|DoOnce false :!label _label
      (:Completed
        (CameraFades|StartCameraFade :self _returnvalue :ToAlpha 1.0 :Duration 2.0)
        (Utilities|FlowControl|Delay 2.0)
        (Transformation|Teleport (Game|Player|GetPlayerPawn 0) (Variables|Default|GetDest%20Location) "0, 0, 0")
        (Class|BPIWeatherSystem|IsInterior(Message) (Game|Player|GetPlayerPawn 0) (Variables|Default|GetIsInterior))
        (CameraFades|StartCameraFade :self _returnvalue :FromAlpha 1.0 :Duration 2.0)
        (Utilities|FlowControl|Delay 5.0)
        (goto _label Reset)))))

(fn ConstructionScript)