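; Inventory component that holds the player's items in an array sized to eight slots and displays them through WB_inventory.
; The inventory input action or Escape toggles the widget, switching cursor, input mode and viewing flag, and notifying the pawn.
; AddItem scans slots in order, stacking matches up to three or filling an empty slot.
; SubstractItem decrements or removes entries, and both functions reload the widget after changes.
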(event Input|EnhancedActionEvents|EnhancedInputActionIA_Inventory
  (params (ActionValue :type Boolean) (ElapsedSeconds :type Float%20%28double-precision%29) (TriggeredSeconds :type Float%20%28double-precision%29) (InputAction :type Input%20Action%20Object%20Reference :default "/Game/Blueprints/Input/Actions/IA_Inventory.IA_Inventory"))
  (bind _returnvalue (Game|GetPlayerController 0))
  (bind _returnvalue_2 (Game|GetPlayerController 0))
  (bind _inventorywidget (Variables|Default|GetInventorywidget))
  (:Started
    (if (Widget|IsVisible (Variables|Default|GetInventorywidget))
      (Default|CloseInvetory (Variables|Default|GetInventorywidget))
      (Utilities|FlowControl|Delay 1.0)
      (Widget|RemovefromParent _inventorywidget)
      (Variables|/Script/Engine.PlayerController|SetbShowMouseCursor _returnvalue false)
      (Variables|Default|SetIsViewing false)
      (Input|SetInputModeGameOnly _returnvalue false)
      (Class|BPIInventory|InsInteract(Message) (Game|Player|GetPlayerPawn 0))
      (else
        (Default|OpenInventory (Variables|Default|GetInventorywidget))
        (Variables|/Script/Engine.PlayerController|SetbShowMouseCursor _returnvalue_2 true)
        (Variables|Default|SetIsViewing true)
        (Input|SetInputModeGameandUI _returnvalue_2 0 "DoNotLock" true false)
        (UserInterface|Viewport|AddtoViewport _inventorywidget 0)
        (Class|BPIInventory|InsInteract(Message) (Game|Player|GetPlayerPawn 0))))))

(event EventBeginPlay
  (UserInterface|CreateWidget "/Game/DevTools/Widget/WB_Debug.WB_Debug_C")
  (bind _returnvalue (UserInterface|CreateWidget "/Game/Blueprints/Inventory/Widget/WB_inventory.WB_inventory_C"))
  (Variables|Default|SetInventorywidget _returnvalue)
  (Utilities|Array|Resize (Variables|Default|GetItems) 8)
  (Default|LoadInventory (Variables|Default|GetInventorywidget) self))

(event Input|KeyboardEvents|Escape
  (params (Key :type Key%20Structure :default "None"))
  (bind _returnvalue (Game|GetPlayerController 0))
  (bind _returnvalue_2 (Game|GetPlayerController 0))
  (bind _inventorywidget (Variables|Default|GetInventorywidget))
  (:Pressed
    (if (Widget|IsVisible (Variables|Default|GetInventorywidget))
      (Default|CloseInvetory (Variables|Default|GetInventorywidget))
      (Utilities|FlowControl|Delay 1.0)
      (Widget|RemovefromParent _inventorywidget)
      (Variables|/Script/Engine.PlayerController|SetbShowMouseCursor _returnvalue false)
      (Variables|Default|SetIsViewing false)
      (Input|SetInputModeGameOnly _returnvalue false)
      (Class|BPIInventory|InsInteract(Message) (Game|Player|GetPlayerPawn 0))
      (else
        (Default|OpenInventory (Variables|Default|GetInventorywidget))
        (Variables|/Script/Engine.PlayerController|SetbShowMouseCursor _returnvalue_2 true)
        (Variables|Default|SetIsViewing true)
        (Input|SetInputModeGameandUI _returnvalue_2 0 "DoNotLock" true false)
        (UserInterface|Viewport|AddtoViewport _inventorywidget 0)
        (Class|BPIInventory|InsInteract(Message) (Game|Player|GetPlayerPawn 0))))))

(fn AddItem
  (params (Item :type S%20Item%20Struct%20Structure))
  (bind (_name _description _weapontype _stackable _quantity) (Utilities|Struct|BreakS_ItemStruct Item))
  (bind (_name_2 _description_2 _weapontype_2 _stackable_2 _quantity_2 _thumnail _mesh _canheal _isinspectitem) (Utilities|Struct|BreakS_ItemStruct Item))
  (bind _items (Variables|Default|GetItems))
  (bind (_array_element _array_index) (Utilities|Array|ForEachLoopwithBreak (Variables|Default|GetItems))
    (:LoopBody
      (if _isinspectitem
        (Variables|Default|SetItemInspectS true)
        (else
          (Variables|Default|SetItemInspectS false)))
      (if _canheal
        (Variables|Default|SetItemHeal true)
        (else
          (Variables|Default|SetItemHeal false)))
      (if (Math|Boolean|ANDBoolean (== (.Name (Utilities|Struct|BreakS_ItemStruct _array_element)) _name) _stackable (<= (+ (.Quantity (Utilities|Struct|BreakS_ItemStruct _array_element)) _quantity) 3))
        (Utilities|Array|SetArrayElem _items _array_index (Utilities|Struct|MakeS_ItemStruct _name_2 _description_2 _weapontype_2 _stackable_2 (+ (.Quantity (Utilities|Struct|BreakS_ItemStruct _array_element)) _quantity) _thumnail _mesh _canheal))
        (Default|LoadInventory (Variables|Default|GetInventorywidget) self :!label _label)
        (return true)
        (elif (== (.Quantity (Utilities|Struct|BreakS_ItemStruct _array_element)) 0)
          (Utilities|Array|SetArrayElem _items _array_index (Utilities|Struct|MakeS_ItemStruct _name_2 _description_2 _weapontype_2 _stackable_2 (+ (.Quantity (Utilities|Struct|BreakS_ItemStruct _array_element)) _quantity) _thumnail _mesh _canheal))
          (goto _label))))))

(fn InsViewing
  (return (Variables|Default|GetIsViewing)))

(fn SubstractItem
  (params (Item :type S%20Item%20Struct%20Structure) (Index :type Integer))
  (bind _quantity (Utilities|Struct|BreakS_ItemStruct Item))
  (bind (_name _description _weapontype _stackable _quantity_2 _thumnail _mesh) (Utilities|Struct|BreakS_ItemStruct Item))
  (bind _items (Variables|Default|GetItems))
  (bind _returnvalue (- _quantity 1))
  (if (<= _returnvalue 0)
    (Utilities|Array|RemoveItem _items Item)
    (else
      (Utilities|Array|SetArrayElem _items Index (Utilities|Struct|MakeS_ItemStruct _name "" _weapontype _stackable _returnvalue _thumnail _mesh))))
  (Default|LoadInventory (Variables|Default|GetInventorywidget) self)
  (return true))