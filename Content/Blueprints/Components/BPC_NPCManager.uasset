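; NPC manager component that periodically spawns NPCs onto splines, up to a maximum count.
; A looping timer started on BeginPlay picks a random NPCSpline entry and fetches its spline through a GetSplineNPCMessage call.
; Each NPC spawns at the spline's first point, read in local space, and receives that spline as a spawn parameter.
; The active count only increments here, and the random index range includes the array length.
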(event Custom|TrySpawnClass
  (bind _npcspline (Variables|Default|GetNPCSpline))
  (if (< (Variables|Default|GetActiveNPCs) (Variables|Default|GetMaxNPCs))
    (bind _getspline (Class|BPINPCSpline|GetSplineNPC(Message) (Utilities|Array|Get(acopy) _npcspline (Math|Random|RandomIntegerinRange 0 (Utilities|Array|Length _npcspline)))))
    (Game|SpawnActorfromClass "/Game/Player_Enemies/Mannequin/NPC/NPC.NPC_C" (Math|Conversions|ToTransform(Vector) (Spline|GetLocationatSplinePoint _getspline 0 "Local")) "Undefined" "MultiplyWithRoot" 0 _getspline 0)
    (Math|Integer|IncrementInt (Variables|Default|GetActiveNPCs))))

(event EventBeginPlay
  (Utilities|Time|SetTimerbyEvent (delegate Custom|TrySpawnClass) (Variables|Default|GetSpawnInterval) true))