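; Dialogue component that shows an array of lines on screen, advancing one line per Talk or Cinematica call.
; Both events share one path that creates a WB_Dialogue widget on the first line and sets its text from TalkIndex, provided NewVar is not valid.
; A call past the last line removes the widget and resets the state.
; Interaction getters return only zero values or the first enum entry.
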(event Custom|Cinematica
  (params (Dialogue :type Array%20of%20Strings))
  (Variables|Default|SetDialogue Dialogue)
  (if (< (Variables|Default|GetTalkIndex) (Utilities|Array|Length (Variables|Default|GetDialogue)))
    (Variables|Default|GetNewVar
      (:then)
      (:else
        (if (Variables|Default|GetActionValue)
          _
          (else
            (bind _returnvalue (UserInterface|CreateWidget "/Game/Blueprints/Widgets/WB_Dialogue.WB_Dialogue_C" (Game|GetPlayerController 0)))
            (bind _output_get (Variables|Default|SetUI _returnvalue))
            (UserInterface|Viewport|AddtoViewport _output_get 0)
            (Variables|Default|SetActionValue true)))
        (Rendering|Components|TextRender|SetText (Variables|/Game/Blueprints/Widgets/WB_Dialogue.WB_Dialogue_C|GetSaldeahibro (Variables|Default|GetUI)) (Utilities|Text|ToText(String) (Utilities|Array|Get(acopy) (Variables|Default|GetDialogue) (Variables|Default|GetTalkIndex))))
        (bind _result (Math|Integer|IncrementInt (Variables|Default|GetTalkIndex))
          (:%20%20
            (Variables|Default|SetTalkIndex _result)))))
    (else
      (Widget|RemovefromParent (Variables|Default|GetUI))
      (Variables|Default|SetTalkIndex 0)
      (Variables|Default|SetActionValue false))))

(event Custom|Talk
  (params (Dialogue :type Array%20of%20Strings))
  (Variables|Default|SetDialogue Dialogue)
  (if (< (Variables|Default|GetTalkIndex) (Utilities|Array|Length (Variables|Default|GetDialogue)))
    (Variables|Default|GetNewVar
      (:then)
      (:else
        (if (Variables|Default|GetActionValue)
          _
          (else
            (bind _returnvalue (UserInterface|CreateWidget "/Game/Blueprints/Widgets/WB_Dialogue.WB_Dialogue_C" (Game|GetPlayerController 0)))
            (bind _output_get (Variables|Default|SetUI _returnvalue))
            (UserInterface|Viewport|AddtoViewport _output_get 0)
            (Variables|Default|SetActionValue true)))
        (Rendering|Components|TextRender|SetText (Variables|/Game/Blueprints/Widgets/WB_Dialogue.WB_Dialogue_C|GetSaldeahibro (Variables|Default|GetUI)) (Utilities|Text|ToText(String) (Utilities|Array|Get(acopy) (Variables|Default|GetDialogue) (Variables|Default|GetTalkIndex))))
        (bind _result (Math|Integer|IncrementInt (Variables|Default|GetTalkIndex))
          (:%20%20
            (Variables|Default|SetTalkIndex _result)))))
    (else
      (Widget|RemovefromParent (Variables|Default|GetUI))
      (Variables|Default|SetTalkIndex 0)
      (Variables|Default|SetActionValue false))))

(fn GetApCount
  (return 0))

(fn GetHoldDuration
  (return 0.0))

(fn GetInteractionLocation
  (return "0, 0, 0"))

(fn GetTypeInteraction
  (return "NewEnumerator0"))