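; BPC_DamgeSystem is an actor component that manages health, healing, damage and death for its owner.
; TakeDamage routes a damage info struct through CanBeDamaged, which checks death, invincibility and blocking to pick blocked, damaged or ignored.
; Event dispatchers report heals, blocks with parry eligibility, deaths and hit responses, the last only when interruptible or forced.
; Heal clamps to max health, and the damage-type dispatcher call is never reached.
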(fn Heal
  (params (Amount :type Float%20%28double-precision%29))
  (if (not (Variables|Default|GetIsDead))
    (bind _output_get (Variables|Default|SetHealth (Math|Float|Clamp(Float) (+ Amount (Variables|Default|GetHealth)) 0.0 (Variables|Default|GetMaxHealth))))
    (Default|CallOnHeal)
    (return _output_get)))

(fn TakeDamage
  (params (DamageInfo :type S%20Damage%20Info%20Structure))
  (bind (_amount _damagetype _damageresponse _shoulddamgeinvincible _canbeblocked _canbeparried _shouldforceinterrupt) (Utilities|Struct|BreakS_DamageInfo DamageInfo))
  (Utilities|CanbeDamaged _shoulddamgeinvincible _canbeblocked
    (:Blocked
      (Development|PrintString "Blocked")
      (Default|CallOnBlocked _canbeparried)
      (return false))
    (:DoDamaged
      (bind _output_get (Variables|Default|SetHealth (- (Variables|Default|GetHealth) _amount)))
      (if (<= _output_get 0.0)
        (Variables|Default|SetIsDead true)
        (Default|CallOnDeath)
        (return true)
        (elif (or (Variables|Default|GetisInterruptible) _shouldforceinterrupt)
          (Default|CallOnDamagedResponse _damageresponse)
          (return true))))
    (:NoDamaged
      (return false))))