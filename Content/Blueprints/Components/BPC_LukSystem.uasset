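; Luk currency and shop component that holds a money balance and lets the player buy items through the WB_Tienda widget.
; OpenShop toggles the widget, cursor and input mode, while SellItems stores the stock and loads it into the widget.
; TakeMoney adds Luks; SellFunction deducts each affordable stock price, not specifically the requested item's, until the player character accepts the item.
; The interaction and balance getters are stubs returning defaults.
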(event EventBeginPlay
  (bind _returnvalue (UserInterface|CreateWidget "/Game/Blueprints/Widgets/Tienda_Luks/WB_Tienda.WB_Tienda_C"))
  (Variables|Default|SetTiendaWidget _returnvalue))

(event EventOpenShop
  (bind _returnvalue (Game|GetPlayerController 0))
  (bind _tiendawidget (Variables|Default|GetTiendaWidget))
  (if (Widget|IsVisible (Variables|Default|GetTiendaWidget))
    (Widget|RemovefromParent _tiendawidget)
    (Variables|/Script/Engine.PlayerController|SetbShowMouseCursor _returnvalue false)
    (Input|SetInputModeGameOnly _returnvalue false)
    (else
      (Variables|/Script/Engine.PlayerController|SetbShowMouseCursor _returnvalue true)
      (Input|SetInputModeGameandUI _returnvalue 0 "DoNotLock" true false)
      (UserInterface|Viewport|AddtoViewport _tiendawidget 0))))

(fn TakeMoney
  (params (Amount :type Integer))
  (bind _output_get (Variables|Default|SetLuks (+ Amount (Variables|Default|GetLuks))))
  (return _output_get))

(fn SellFunction
  (params (SellItem :type S%20Item%20Struct%20Structure))
  (bind _array_element (Utilities|Array|ForEachLoopwithBreak (Variables|Default|GetItems))
    (:LoopBody
      (if (> (Variables|Default|GetLuks) (.Precio (Utilities|Struct|BreakS_ItemStruct _array_element)))
        (bind _output_get (Variables|Default|SetLuks (- (Variables|Default|GetLuks) (.Precio (Utilities|Struct|BreakS_ItemStruct _array_element)))))
        (bind _wasaded (Class|BPIInventory|AddItem(Message) (Game|GetPlayerCharacter 0) SellItem))
        (if _wasaded
          (Development|PrintString "Si vendio")
          (Development|PrintString (Utilities|String|ToString(Integer) _output_get))
          (return _wasaded))))))

(fn SellItems
  (params (Items :type Array%20of%20S%20Item%20Struct%20Structures))
  (bind _output_get (Variables|Default|SetItems Items))
  (Default|LoadSellItems (Variables|Default|GetTiendaWidget) self _output_get))

(fn CurrentLuks
  (return 0))

(fn GetApCount
  (return 0))

(fn GetHoldDuration
  (return 0.0))

(fn GetInteractionLocation
  (return "0, 0, 0"))

(fn GetLuks
  (params (Luks :type Integer))
  (return 0))

(fn GetTypeInteraction
  (return "NewEnumerator0"))