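; BPC_NPCSpawner is a component that spawns an NPC near its owner, set off by a timer started on BeginPlay.
; While SpawnedNPCs is under MaxNPCs, it picks a random X offset from SpawnRadius and line-traces vertically with debug drawing.
; A hit on a "Floor"-tagged actor spawns the NPC there, passing it the owner and radius.
; New NPCs are never added to SpawnedNPCs, and the array's cleanup loop is unwired.
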(event Custom|OlaTry
  (CallFunction|TrySpawnNPC))

(event EventBeginPlay
  (Utilities|Time|SetTimerbyEvent (delegate Custom|OlaTry) (Variables|Default|GetSpawnInterval)))

(fn TrySpawnNPC
  (bind _spawnradius (Variables|Default|GetSpawnRadius))
  (if (< (Utilities|Array|Length (Variables|Default|GetSpawnedNPCs)) (Variables|Default|GetMaxNPCs))
    (Variables|Default|SetOwnerLocation (Transformation|GetActorLocation (Components|GetOwner)))
    (bind _result (Math|Float|NegateFloat _spawnradius)
      (:%20%20
        (Variables|Default|SetRandX (Math|Random|RandomFloatinRange _result _spawnradius))
        (Variables|Default|SetTraceStart (+ (Math|Vector|MakeVector (Variables|Default|GetRandX) 0.0 2e+02) (Variables|Default|GetOwnerLocation)))
        (Variables|Default|SetTraceEnd (+ (Math|Vector|MakeVector (Variables|Default|GetRandX) 0.0 -2e+02) (Variables|Default|GetOwnerLocation)))
        (bind _outhit (Collision|LineTraceByChannel (Variables|Default|GetTraceStart) (Variables|Default|GetTraceEnd) "TraceTypeQuery1" false 0 "ForDuration"))
        (if (Actor|ActorHasTag (.HitActor (Collision|BreakHitResult _outhit)) "Floor")
          (bind _returnvalue (Game|SpawnActorfromClass "/Game/Player_Enemies/Mannequin/NPC/NPC.NPC_C" (Math|Conversions|ToTransform(Vector) (.Location (Collision|BreakHitResult _outhit))) "Undefined" "MultiplyWithRoot" 0 0))
          (Class|BPINPC|InitNPC(Message) _returnvalue (Components|GetOwner) (Variables|Default|GetSpawnRadius))
          (else
            (return)))))))