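; BP_Hint is an interactable clue pickup placed in the world that plays a sound from BeginPlay.
; The construction script sets its mesh from the ItemStruct data and disables physics simulation.
; On interaction it passes the ItemStruct to the interactor's AddItemMessage, and on success stops the sound and destroys itself.
; Its interaction query functions return fixed defaults, including zero AP count and zero hold duration.
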(event EventInteracti
  (params (Interactor :type Actor%20Object%20Reference))
  (bind _wasaded (Class|BPIInventory|AddItem(Message) Interactor (Variables|Default|GetItemStruct)))
  (if _wasaded
    (Audio|Components|Audio|Stop (Variables|Default|GetSonido))
    (Actor|DestroyActor)))

(event EventBeginPlay
  (Audio|Components|Audio|Play (Variables|Default|GetSonido) 0.0))

(fn ConstructionScript
  (bind _staticmesh (Variables|Default|GetStaticMesh))
  (Components|StaticMesh|SetStaticMesh _staticmesh (.Mesh (Utilities|Struct|BreakS_ItemStruct (Variables|Default|GetItemStruct))))
  (Physics|SetSimulatePhysics _staticmesh false))

(fn GetApCount
  (return 0))

(fn GetHoldDuration
  (return 0.0))

(fn GetInteractionLocation
  (return "0, 0, 0"))

(fn GetTypeInteraction
  (return "NewEnumerator0"))