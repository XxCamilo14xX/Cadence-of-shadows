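; BP_item is a pickup actor that an interactor can collect.
; Its construction script applies the mesh from its Item data to the static mesh component and disables physics simulation.
; On Interacti it offers the Item to the interactor through an AddItem message and destroys itself only if that returns true.
; The remaining interaction and inventory functions are stubs returning fixed defaults.
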(event EventInteracti
  (params (Interactor :type Actor%20Object%20Reference))
  (bind _wasaded (Class|BPIInventory|AddItem(Message) Interactor (Variables|Default|GetItem)))
  (if _wasaded
    (Actor|DestroyActor)))

(fn ConstructionScript
  (bind _staticmesh (Variables|Default|GetStaticMesh))
  (Components|StaticMesh|SetStaticMesh _staticmesh (.Mesh (Utilities|Struct|BreakS_ItemStruct (Variables|Default|GetItem))))
  (Physics|SetSimulatePhysics _staticmesh false))

(fn AddItem
  (params (Item :type S%20Item%20Struct%20Structure))
  (return false))

(fn GetApCount
  (return 0))

(fn GetHoldDuration
  (return 0.0))

(fn GetInteractionLocation
  (return "0, 0, 0"))

(fn GetTypeInteraction
  (return "NewEnumerator0"))

(fn InsViewing
  (return false))

(fn SubstractItem
  (params (Item :type S%20Item%20Struct%20Structure) (Index :type Integer))
  (return false))