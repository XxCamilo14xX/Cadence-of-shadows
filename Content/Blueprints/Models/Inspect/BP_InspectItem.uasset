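; Inspectable item actor that shows its own mesh, or one passed in an item struct, in an inspection UI.
; Construction copies the mesh to InsMesh 10,000 units below, where a SceneCapture2D renders only that component.
; Inspecting opens the widget, switches input context and registers with BP_PlayerController, while events move, rotate and FOV-zoom the mesh.
; Exiting resets the view, restores game input and destroys the actor.
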(event Custom|UpdateMeshRotation
  (params (Vector%202D :type Vector%202D%20Structure))
  (bind (_x _y) (Math|Vector2D|BreakVector2D Vector%202D))
  (bind _insmesh (Variables|Default|GetInsMesh))
  ;[0.15 0.15 0.15 0.5] Rotation
  (Transformation|SetRelativeRotation _insmesh (Math|Rotator|CombineRotators (Variables|/Script/Engine.SceneComponent|GetRelativeRotation _insmesh) (Math|Rotator|MakeRotator (* _y -5.0) 0.0 (* _x -5.0))) false false))

(event Custom|UpdateMeshLocation
  (params (Vector2D :type Vector%202D%20Structure))
  (bind (_x _y) (Math|Vector2D|BreakVector2D Vector2D))
  ;[0.15 0.15 0.15 0.5] Location
  (Transformation|SetRelativeLocation (Variables|Default|GetInsMesh) (Math|Vector|MakeVector (+ (.x (Variables|/Script/Engine.SceneComponent|GetRelativeLocation (Variables|Default|GetInsMesh))) (* _x 2.0)) 0.0 (+ (.z (Variables|/Script/Engine.SceneComponent|GetRelativeLocation (Variables|Default|GetInsMesh))) (* _y 2.0))) false false))

(event Custom|ExitInspectionMode
  (bind _returnvalue (Game|GetPlayerController 0))
  ;[0.15 0.15 0.15 0.5] Exit Inspect Mode
  (Development|SetHiddeninGame (Variables|Default|GetInsMesh) true false)
  (CallFunction|ResetDefault)
  (Widget|RemovefromParent (Variables|Default|GetInspectUI))
  (Variables|/Script/Engine.PlayerController|SetbShowMouseCursor _returnvalue true)
  (Input|SetInputModeGameOnly _returnvalue false)
  (bind _asbp_player_controller (Utilities|Casting|CastToBP_PlayerController (Game|GetPlayerController 0)))
  (Default|UpdateInputMapContext _asbp_player_controller "/Game/Blueprints/Input/IMC_Hybrid.IMC_Hybrid")
  (Actor|DestroyActor))

(event Custom|ResetDefault
  ;[0.15 0.15 0.15 0.5] Exit Inspect Mode
  (Transformation|SetRelativeTransform (Variables|Default|GetInsMesh) (Variables|Default|GetDefaultPos) false false)
  (Variables|/Script/Engine.SceneCaptureComponent2D|SetFOVAngle (Variables|Default|GetSceneCaptureComponent2D) 9e+01)
  (Class|SceneCaptureComponent|SetCaptureSortPriority (Variables|Default|GetSceneCaptureComponent2D) 1))

(event Custom|UpdateMeshZoom
  (params (Axis :type Float%20%28double-precision%29))
  (bind _scenecapturecomponent2d (Variables|Default|GetSceneCaptureComponent2D))
  ;[0.15 0.15 0.15 0.5] Zoom
  (bind _output_get (Variables|/Script/Engine.SceneCaptureComponent2D|SetFOVAngle _scenecapturecomponent2d (Math|Float|Clamp(Float) (+ (Variables|/Script/Engine.SceneCaptureComponent2D|GetFOVAngle _scenecapturecomponent2d) (* Axis -3.0)) 1e+01 1.2e+02)))
  (Development|PrintString (Utilities|String|ToString(Float) _output_get)))

(event EventInspectItemClik
  (params (SItemStruct :type S%20Item%20Struct%20Structure))
  (bind _returnvalue (Game|GetPlayerController 0))
  (Components|StaticMesh|SetStaticMesh (Variables|Default|GetInsMesh) (.Mesh (Utilities|Struct|BreakS_ItemStruct SItemStruct)))
  (Class|SceneCaptureComponent|SetCaptureSortPriority (Variables|Default|GetSceneCaptureComponent2D))
  (Development|SetHiddeninGame (Variables|Default|GetInsMesh) false false)
  (bind _returnvalue_2 (UserInterface|CreateWidget "/Game/Blueprints/Models/Inspect/WB_InspectUI.WB_InspectUI_C"))
  (bind _output_get (Variables|Default|SetInspectUI _returnvalue_2))
  (UserInterface|Viewport|AddtoViewport _output_get 0)
  (Variables|/Script/Engine.PlayerController|SetbShowMouseCursor _returnvalue true)
  (Input|SetInputModeGameandUI _returnvalue 0 "DoNotLock" true false)
  (bind _asbp_player_controller (Utilities|Casting|CastToBP_PlayerController (Game|GetPlayerController 0)))
  (Default|UpdateInputMapContext _asbp_player_controller "/Game/Blueprints/Input/IMC_InspectInventory.IMC_InspectInventory")
  (Variables|/Game/Blueprints/BP_PlayerController.BP_PlayerController_C|SetInspectBP _asbp_player_controller self))

(event EventInteracti
  (params (Interactor :type Actor%20Object%20Reference))
  (bind _returnvalue (Game|GetPlayerController 0))
  (Class|SceneCaptureComponent|SetCaptureSortPriority (Variables|Default|GetSceneCaptureComponent2D))
  (Development|SetHiddeninGame (Variables|Default|GetInsMesh) false false)
  (bind _returnvalue_2 (UserInterface|CreateWidget "/Game/Blueprints/Models/Inspect/WB_InspectUI.WB_InspectUI_C"))
  (bind _output_get (Variables|Default|SetInspectUI _returnvalue_2))
  (UserInterface|Viewport|AddtoViewport _output_get 0)
  (Variables|/Script/Engine.PlayerController|SetbShowMouseCursor _returnvalue true)
  (Input|SetInputModeGameandUI _returnvalue 0 "DoNotLock" true false)
  (bind _asbp_player_controller (Utilities|Casting|CastToBP_PlayerController (Game|GetPlayerController 0)))
  (Default|UpdateInputMapContext _asbp_player_controller "/Game/Blueprints/Input/IMC_InspectInventory.IMC_InspectInventory")
  (Variables|/Game/Blueprints/BP_PlayerController.BP_PlayerController_C|SetInspectBP _asbp_player_controller self))

(fn ConstructionScript
  (bind _staticmesh (Variables|Default|GetStaticMesh))
  (bind _insmesh (Variables|Default|GetInsMesh))
  (bind _scenecapturecomponent2d (Variables|Default|GetSceneCaptureComponent2D))
  (bind _relativelocation (Variables|/Script/Engine.SceneComponent|GetRelativeLocation _scenecapturecomponent2d))
  (bind _relativelocation_2 (Variables|/Script/Engine.SceneComponent|GetRelativeLocation _insmesh))
  (|CallParentFunction)
  (Rendering|SceneCapture|ShowOnlyComponent (Variables|Default|GetSceneCaptureComponent2D) (Variables|Default|GetInsMesh))
  (Components|StaticMesh|SetStaticMesh _insmesh (Variables|/Script/Engine.StaticMeshComponent|GetStaticMesh _staticmesh))
  (Transformation|SetRelativeTransform _insmesh (Transformation|GetRelativeTransform _staticmesh) false false)
  (Transformation|SetRelativeLocation _insmesh (Math|Vector|MakeVector (.x _relativelocation_2) (.y _relativelocation_2) -1e+04) false false)
  (Transformation|SetRelativeLocation _scenecapturecomponent2d (Math|Vector|MakeVector (.x _relativelocation) (.y _relativelocation) -1e+04) false false)
  (Variables|Default|SetDefaultPos (Transformation|GetRelativeTransform (Variables|Default|GetInsMesh))))