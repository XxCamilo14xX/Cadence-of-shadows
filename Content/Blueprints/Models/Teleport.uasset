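; Interactable teleporter Blueprint that moves whoever interacts with it to a destination based on its Sphere component.
; The interact event teleports the interactor to the Sphere's world location plus an X/Y offset, resets its rotation to zero and prints a debug string.
; Interaction getters for AP count, hold duration, location and type return only zero values or the first enum entry.
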(event EventInteracti
  (params (Interactor :type Actor%20Object%20Reference))
  (Transformation|Teleport Interactor (+ (Transformation|GetWorldLocation (Variables|Default|GetSphere)) (Math|Vector|MakeVector (Variables|Default|GetX) (Variables|Default|GetY) 0.0)) "0, 0, 0")
  (Development|PrintString "TP"))

(fn ConstructionScript)

(fn GetApCount
  (return 0))

(fn GetHoldDuration
  (return 0.0))

(fn GetInteractionLocation
  (return "0, 0, 0"))

(fn GetTypeInteraction
  (return "NewEnumerator0"))