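; BP_TableroItems is an interactable board (tablero) that opens an inventory inspection UI and displays dropped clue items as 3D meshes.
; Interacting shows the TableroWidget from the interactor's BPC_Inventory, enables the cursor with game-and-UI input, and switches to the inspect-inventory mapping context.
; Dropping an item spawns a BP_ClueMeshActor with the item's mesh at the drop location.
; Each drop replaces the SceneCapture2D show-only list with just that new actor.
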(event EventDroppedItem
  (params (ItemData :type S%20Item%20Struct%20Structure) (DropLocation :type Vector :default "0, 0, 0"))
  (bind _returnvalue (Game|SpawnActorfromClass "/Game/Blueprints/Models/Tablero/BP_ClueMeshActor.BP_ClueMeshActor_C" (Math|Transform|MakeTransform DropLocation "0, 0, 0" "1.000000,1.000000,1.000000") "Undefined" "MultiplyWithRoot" 0 0))
  (Components|StaticMesh|SetStaticMesh (Variables|/Game/Blueprints/Models/Tablero/BP_ClueMeshActor.BP_ClueMeshActor_C|GetStaticMesh _returnvalue) (.Mesh (Utilities|Struct|BreakS_ItemStruct ItemData)))
  (bind _output_get (Variables|Default|SetShownCaptureActors (Utilities|Array|MakeArray _returnvalue)))
  (Variables|/Script/Engine.SceneCaptureComponent|SetShowOnlyActors (Variables|Default|GetSceneCaptureComponent2D) _output_get))

(event EventInteracti
  (params (Interactor :type Actor%20Object%20Reference))
  (bind _returnvalue (Game|GetPlayerController 0))
  (Class|SceneCaptureComponent|SetCaptureSortPriority (Variables|Default|GetSceneCaptureComponent2D))
  (bind _output_get (Variables|Default|SetInspectUI (Variables|/Game/Blueprints/Components/BPC_Inventory.BPC_Inventory_C|GetTableroWidget (Actor|GetComponentbyClass Interactor "/Game/Blueprints/Components/BPC_Inventory.BPC_Inventory_C"))))
  (UserInterface|Viewport|AddtoViewport _output_get 0)
  (Variables|/Script/Engine.PlayerController|SetbShowMouseCursor _returnvalue true)
  (Input|SetInputModeGameandUI _returnvalue 0 "DoNotLock" true false)
  (bind _asbp_player_controller (Utilities|Casting|CastToBP_PlayerController (Game|GetPlayerController 0)))
  (Default|UpdateInputMapContext _asbp_player_controller "/Game/Blueprints/Input/IMC_InspectInventory.IMC_InspectInventory"))

(fn ConstructionScript)

(fn GetApCount
  (return 0))

(fn GetHoldDuration
  (return 0.0))

(fn GetInteractionLocation
  (return "0, 0, 0"))

(fn GetTypeInteraction
  (return "NewEnumerator0"))