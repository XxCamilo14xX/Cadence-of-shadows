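; BP_NPCCar is an NPC traffic car that moves along road points supplied by its owning spline.
; Traffic-light changes map to Driving, Slowing or Stopped states; a Hit Player state also halts it.
; UpdateCarPosition runs on BeginPlay or the continue event, sweeping the car to the spline's current road point and incrementing it.
; Speed values are stored but don't drive movement; distance-based advance and rotation logic are disconnected.
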(event Custom|continue
  (CallFunction|UpdateCarPosition (Variables|Default|GetSplineOwner)))

(event EventBeginPlay
  (CallFunction|UpdateCarPosition (Variables|Default|GetSplineOwner)))

(event EventOnTrafficStateChanged
  (params (NewState :type E_TrafficState%20Enum :default "NewEnumerator0"))
  (switch Utilities|FlowControl|Switch|SwitchonE_TrafficState NewState
    (:NewEnumerator0
      (Variables|Default|SetCurrentState "NewEnumerator0"))
    (:NewEnumerator1
      (Variables|Default|SetCurrentState "NewEnumerator1"))
    (:NewEnumerator2
      (Variables|Default|SetCurrentState "NewEnumerator2"))))

(fn ConstructionScript)

(fn UpdateCarPosition
  (params (Spline :type BP%20Spline%20Road%20Object%20Reference))
  (switch Utilities|FlowControl|Switch|SwitchonE_CarState (Variables|Default|GetCurrentState)
    (:NewEnumerator0
      (bind _output_get (Variables|Default|SetCarData (Utilities|Struct|MakeS_CarData (.currentspeed (Variables|Default|GetCarData)) (.maxspeed (Variables|Default|GetCarData)) (.splinedistance (Variables|Default|GetCarData)) (.splineref (Variables|Default|GetCarData)))))
      (Variables|Default|SetCurrent%20Speed (.currentspeed _output_get))
      (Variables|Default|SetMax%20Speed (.maxspeed _output_get))
      (Variables|Default|SetbIsMoving%20 true)
      (bind _location (Default|GetRoadPointPosition Spline :!label _label))
      (Transformation|SetActorLocation _location true false)
      (Default|IncrementRoad Spline)
      (if (>= (.splinedistance (Variables|Default|GetCarData)) 0.0)
        _))
    (:NewEnumerator1
      (Variables|Default|SetCarData (Utilities|Struct|MakeS_CarData (Math|Float|Lerp (Variables|Default|GetCurrent%20Speed) (* (Variables|Default|GetMax%20Speed) 0.3) 0.05) 6e+02 0.0 0))
      (Variables|Default|SetbIsMoving%20 true)
      (goto _label))
    (:NewEnumerator2
      (Variables|Default|SetCarData (Utilities|Struct|MakeS_CarData 0.0 6e+02 0.0 0))
      (Variables|Default|SetbIsMoving%20 false))
    (:NewEnumerator3
      (Variables|Default|SetCarData (Utilities|Struct|MakeS_CarData 0.0 6e+02 0.0 0))
      (Variables|Default|SetbIsMoving%20 false))))