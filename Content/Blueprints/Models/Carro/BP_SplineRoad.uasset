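; BP_SplineRoad is a road path actor that exposes the points of a spline one at a time as world positions.
; IncrementRoad advances RoadIndex by Direction and wraps it to zero when it equals the spline's point count.
; GetRoadPointPosition returns the world location of the spline point at the current RoadIndex.
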(event Custom|IncrementRoad
  (bind _output_get (Variables|Default|SetRoadIndex (+ (Variables|Default|GetRoadIndex) (Variables|Default|GetDirection))))
  (if (== _output_get (Spline|GetNumberOfSplinePoints (Variables|Default|GetSpline)))
    (Variables|Default|SetRoadIndex 0)))

(fn ConstructionScript)

(fn GetRoadPointPosition
  (return (Spline|GetLocationatSplinePoint (Variables|Default|GetSpline) (Variables|Default|GetRoadIndex) "World")))