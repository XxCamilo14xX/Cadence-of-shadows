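; BP_TrafficLight is a traffic light that cycles through green, yellow and red phases, starting on green at BeginPlay.
; Each phase function sets CurrentState, prints it, and chains to the next phase with a timer using that phase's duration.
; On every change it sends the new state through BPI_TrafficListener to implementing actors overlapping IntersectionZone, so only actors inside at that moment are notified.
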(event EventBeginPlay
  (CallFunction|StartGreenPhase))

(fn ConstructionScript)

(fn StartGreenPhase
  (bind _output_get (Variables|Default|SetCurrentState "NewEnumerator0"))
  (Development|PrintString (Utilities|String|EnumtoString _output_get))
  (CallFunction|NotifyCarsNearby)
  (Utilities|Time|SetTimerbyFunctionName 0 "StartYellowPhase" (Variables|Default|GetGreenDuration)))

(fn NotifyCarsNearby
  (for _array_element (Collision|GetOverlappingActors (Variables|Default|GetIntersectionZone) 0 :!class /Script/Engine.PrimitiveComponent)
    (if (Utilities|DoesObjectImplementInterface _array_element "/Game/Blueprints/Models/Carro/BPI_TrafficListener.BPI_TrafficListener_C")
      (Class|BPITrafficListener|OnTrafficStateChanged(Message) _array_element (Variables|Default|GetCurrentState)))))

(fn StartYellowPhase
  (bind _output_get (Variables|Default|SetCurrentState "NewEnumerator1"))
  (Development|PrintString (Utilities|String|EnumtoString _output_get))
  (CallFunction|NotifyCarsNearby)
  (Utilities|Time|SetTimerbyFunctionName 0 "StartRedPhase" (Variables|Default|GetYellowDuration)))

(fn StartRedPhase
  (bind _output_get (Variables|Default|SetCurrentState "NewEnumerator2"))
  (Development|PrintString (Utilities|String|EnumtoString _output_get))
  (CallFunction|NotifyCarsNearby)
  (Utilities|Time|SetTimerbyFunctionName 0 "StartGreenPhase" (Variables|Default|GetRedDuration)))