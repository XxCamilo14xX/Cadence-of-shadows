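; BP_TPTrigger is a teleport trigger that stays inactive until game progression unlocks it.
; It binds to the game instance's progression event, then arms itself and shows its point light when the action target matches its TargetID, with a switch on StepID.
; Once armed, any overlap with its sphere teleports player pawn 0 to a hard-coded location, without checking which actor overlapped.
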(event OnComponentBeginOverlap(Sphere)
  (params (OverlappedComponent :type Primitive%20Component%20Object%20Reference) (OtherActor :type Actor%20Object%20Reference) (OtherComp :type Primitive%20Component%20Object%20Reference) (OtherBodyIndex :type Integer) (bFromSweep :type Boolean) (SweepResult :type Hit%20Result%20Structure%20%28by%20ref%29))
  (if (Variables|Default|GetYa)
    (Transformation|Teleport (Game|Player|GetPlayerPawn 0) "700.000000,-3890.000000,50.000000" "0, 0, 0")))

(event Custom|ChaoPorta
  (params (StepID :type Name) (ActionTarget :type Name))
  (if (== ActionTarget (Variables|Default|GetTargetID))
    (switch name StepID
      (:Default
        (Variables|Default|SetYa true)
        (Rendering|SetVisibility (Variables|Default|GetPointLight) true false)))))

(event EventBeginPlay
  (EventDispatchers|BindEventtoOnProgresionEvent (CallFunction|GetMyGameInstance) (delegate Custom|ChaoPorta)))

(fn ConstructionScript)