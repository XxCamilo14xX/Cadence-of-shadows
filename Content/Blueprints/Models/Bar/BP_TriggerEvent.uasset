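; BP_TriggerEvent is a Bar trigger actor that starts a dialogue cinematic when something begins overlapping its sphere.
; The overlap passes its Dialogue to BPCTalkSystem's Cinematica and calls Holaa on the map widget, with no filter on the overlapping actor.
; Its interaction functions for location, AP count, hold duration and type return only default values.
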(event OnComponentBeginOverlap(Sphere)
  (params (OverlappedComponent :type Primitive%20Component%20Object%20Reference) (OtherActor :type Actor%20Object%20Reference) (OtherComp :type Primitive%20Component%20Object%20Reference) (OtherBodyIndex :type Integer) (bFromSweep :type Boolean) (SweepResult :type Hit%20Result%20Structure%20%28by%20ref%29))
  (Default|Cinematica (Variables|Default|GetBPC_TalkSystem) (Variables|Default|GetDialogue))
  (Default|Holaa (Variables|Default|GetWBMap)))

(fn ConstructionScript)

(fn GetInteractionLocation
  (return "0, 0, 0"))

(fn GetApCount
  (return 0))

(fn GetHoldDuration
  (return 0.0))

(fn GetTypeInteraction
  (return "NewEnumerator0"))