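; Player controller that routes Enhanced Input actions to the player pawn, its interaction component, an inspection object and the map widget.
; Movement, dash, melee and heal go to the pawn as messages, while interaction press phases drive the component cached at BeginPlay.
; In inspect mode, held mouse buttons gate mesh rotation and movement, and the wheel zooms.
; A custom event swaps mapping contexts; item and map functions are empty stubs.
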(event Custom|UpdateInputMapContext
  (params (InputPin :type Input%20Mapping%20Context%20Object%20Reference))
  (bind _returnvalue (Game|GetPlayerController 0))
  (bind _returnvalue_2 (PlayerController|LocalPlayerSubsystems|GetEnhancedInputLocalPlayerSubsystem _returnvalue))
  ;[0.15 0.15 0.15 0.5] Inputs
  (Utilities|IsValid _returnvalue_2
    (:Is%20Valid
      (Class|EnhancedInputSubsystemInterface|ClearAllMappings _returnvalue_2)
      (Input|AddMappingContext _returnvalue_2 InputPin 0 "(bIgnoreAllPressedKeysUntilRelease=True,bForceImmediately=False,bNotifyUserSettings=False)"))))

(event Input|EnhancedActionEvents|EnhancedInputActionIA_Heal
  (params (ActionValue :type Boolean) (ElapsedSeconds :type Float%20%28double-precision%29) (TriggeredSeconds :type Float%20%28double-precision%29) (InputAction :type Input%20Action%20Object%20Reference :default "/Game/Blueprints/Input/Actions/IA_Heal.IA_Heal"))
  (:Started
    (Class|BPIMoveSet|Healing(Message) (Game|Player|GetPlayerPawn 0))))

(event Input|EnhancedActionEvents|EnhancedInputActionIA_Map
  (params (ActionValue :type Boolean) (ElapsedSeconds :type Float%20%28double-precision%29) (TriggeredSeconds :type Float%20%28double-precision%29) (InputAction :type Input%20Action%20Object%20Reference :default "/Game/Blueprints/Input/Actions/IA_Map.IA_Map"))
  (:Started
    (Default|Map (Variables|Default|GetMiniMapWB))))

(event Input|EnhancedActionEvents|EnhancedInputActionIA_ExitInspect
  (params (ActionValue :type Boolean) (ElapsedSeconds :type Float%20%28double-precision%29) (TriggeredSeconds :type Float%20%28double-precision%29) (InputAction :type Input%20Action%20Object%20Reference :default "/Game/Blueprints/Input/Actions/InspectionInputActions/IA_ExitInspect.IA_ExitInspect"))
  ;[0.15 0.15 0.15 0.5] Inspect Mode
  (:Started
    (Default|ExitInspectionMode (Variables|Default|GetInspectBP))))

(event Input|EnhancedActionEvents|EnhancedInputActionIA_Interaction
  (params (ActionValue :type Boolean) (ElapsedSeconds :type Float%20%28double-precision%29) (TriggeredSeconds :type Float%20%28double-precision%29) (InputAction :type Input%20Action%20Object%20Reference :default "/Game/Blueprints/Input/Actions/IA_Interaction.IA_Interaction"))
  (bind _playerinteraction (Variables|Default|GetPlayerInteraction))
  ;[0.15 0.15 0.15 0.5] Interactions
  (:Started
    (Default|InteractionBegin _playerinteraction))
  (:Ongoing
    (Default|CallOnInteractPressOngoing _playerinteraction ElapsedSeconds))
  (:Canceled
    (EventDispatchers|UnbindallEventsfromOnInteractPressOngoing _playerinteraction :!label _label)
    (Default|CallOnInteractEnded _playerinteraction))
  (:Completed
    (goto _label)))

(event Input|EnhancedActionEvents|EnhancedInputActionIA_Move
  (params (ActionValue :type Vector%202D%20Structure) (ElapsedSeconds :type Float%20%28double-precision%29) (TriggeredSeconds :type Float%20%28double-precision%29) (InputAction :type Input%20Action%20Object%20Reference :default "/Game/Blueprints/Input/Actions/IA_Move.IA_Move"))
  ;[0.05098 0.05098 0.05098] Movement
  (Class|BPIMoveSet|Move(Message) (Game|Player|GetPlayerPawn 0) ActionValue))

(event Input|EnhancedActionEvents|EnhancedInputActionIA_dash
  (params (ActionValue :type Boolean) (ElapsedSeconds :type Float%20%28double-precision%29) (TriggeredSeconds :type Float%20%28double-precision%29) (InputAction :type Input%20Action%20Object%20Reference :default "/Game/Blueprints/Input/Actions/IA_dash.IA_dash"))
  ;[0.05098 0.05098 0.05098] Dash Input
  (:Started
    (Class|BPIMoveSet|Dash(Message) (Game|Player|GetPlayerPawn 0))))

(event Input|EnhancedActionEvents|EnhancedInputActionIA_RightClick
  (params (ActionValue :type Boolean) (ElapsedSeconds :type Float%20%28double-precision%29) (TriggeredSeconds :type Float%20%28double-precision%29) (InputAction :type Input%20Action%20Object%20Reference :default "/Game/Blueprints/Input/Actions/InspectionInputActions/IA_RightClick.IA_RightClick"))
  ;[0.15 0.15 0.15 0.5] Inspect Mode
  (:Triggered
    (Variables|Default|SetRightClickActive true))
  (:Completed
    (Variables|Default|SetRightClickActive false)))

(event Input|EnhancedActionEvents|EnhancedInputActionIA_Attack
  (params (ActionValue :type Boolean) (ElapsedSeconds :type Float%20%28double-precision%29) (TriggeredSeconds :type Float%20%28double-precision%29) (InputAction :type Input%20Action%20Object%20Reference :default "/Game/Blueprints/Input/Actions/IA_Attack.IA_Attack"))
  ;[0.15 0.15 0.15 0.5] Attack
  (:Started
    (Class|BPIMoveSet|Melee(Message) (Game|Player|GetPlayerPawn 0))))

(event Input|EnhancedActionEvents|EnhancedInputActionIA_MouseWheel
  (params (ActionValue :type Float%20%28double-precision%29) (ElapsedSeconds :type Float%20%28double-precision%29) (TriggeredSeconds :type Float%20%28double-precision%29) (InputAction :type Input%20Action%20Object%20Reference :default "/Game/Blueprints/Input/Actions/InspectionInputActions/IA_MouseWheel.IA_MouseWheel"))
  ;[0.15 0.15 0.15 0.5] Inspect Mode
  (Default|UpdateMeshZoom (Variables|Default|GetInspectBP) ActionValue))

(event Input|EnhancedActionEvents|EnhancedInputActionIA_MouseMove
  (params (ActionValue :type Vector%202D%20Structure) (ElapsedSeconds :type Float%20%28double-precision%29) (TriggeredSeconds :type Float%20%28double-precision%29) (InputAction :type Input%20Action%20Object%20Reference :default "/Game/Blueprints/Input/Actions/InspectionInputActions/IA_MouseMove.IA_MouseMove"))
  (bind _inspectbp (Variables|Default|GetInspectBP))
  ;[0.15 0.15 0.15 0.5] Inspect Mode
  (Utilities|FlowControl|Sequence
    (:then_0
      (if (Variables|Default|GetLeftClickActive)
        (Default|UpdateMeshRotation _inspectbp ActionValue)))
    (:then_1
      (if (Variables|Default|GetRightClickActive)
        (Default|UpdateMeshLocation _inspectbp ActionValue)))))

(event Input|EnhancedActionEvents|EnhancedInputActionIA_LeftClick
  (params (ActionValue :type Boolean) (ElapsedSeconds :type Float%20%28double-precision%29) (TriggeredSeconds :type Float%20%28double-precision%29) (InputAction :type Input%20Action%20Object%20Reference :default "/Game/Blueprints/Input/Actions/InspectionInputActions/IA_LeftClick.IA_LeftClick"))
  ;[0.15 0.15 0.15 0.5] Inspect Mode
  (:Triggered
    (Variables|Default|SetLeftClickActive true))
  (:Completed
    (Variables|Default|SetLeftClickActive false)))

(event EventBeginPlay
  (Variables|Default|SetPlayerInteraction (Actor|GetComponentbyClass (Pawn|GetControlledPawn) "/Game/Blueprints/Components/BPC_Interaction_Systemm.BPC_Interaction_Systemm_C"))
  (bind _returnvalue (UserInterface|CreateWidget "/Game/Blueprints/systems/MiniMap/WB_Map.WB_Map_C"))
  (Variables|Default|SetMiniMapWB _returnvalue))

(fn ConstructionScript)

(fn AddItem
  (params (Item :type S%20Item%20Struct%20Structure))
  (return false))

(fn GetMap
  (params (Maapp :type WB%20Map%20Object%20Reference))
  (return))

(fn InsViewing
  (return false))

(fn SubstractItem
  (params (Item :type S%20Item%20Struct%20Structure) (Index :type Integer))
  (return false))