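; BP_NPCManager spawns NPCs onto splines over time, up to a maximum count.
; A looping timer started on BeginPlay picks a random NPCSpline entry and retrieves its spline through GetSplineNPCMessage.
; A valid spline gives the spawn location at its first point and is passed to the new actor, incrementing ActiveNPCs.
; An invalid spline triggers an immediate recursive retry; the count is never decremented here.
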(event Custom|TrySpawnClass
  (bind _npcspline (Variables|Default|GetNPCSpline))
  (if (< (Variables|Default|GetActiveNPCs) (Variables|Default|GetMaxNPCs))
    (bind _getspline (Class|BPINPCSpline|GetSplineNPC(Message) (Utilities|Array|Get(acopy) _npcspline (Math|Random|RandomIntegerinRange 0 (- (Utilities|Array|Length _npcspline) 1)))))
    (Utilities|IsValid _getspline
      (:Is%20Valid
        (Game|SpawnActorfromClass "/Game/Player_Enemies/Mannequin/NPC/NPC.NPC_C" (Math|Conversions|ToTransform(Vector) (Spline|GetLocationatSplinePoint _getspline 0 "World")) "Undefined" "MultiplyWithRoot" 0 (Variables|Default|GetCanSpawn) _getspline 0)
        (Math|Integer|IncrementInt (Variables|Default|GetActiveNPCs)))
      (:Is%20Not%20Valid
        (CallFunction|TrySpawnClass)))))

(event EventBeginPlay
  (Utilities|Time|SetTimerbyEvent (delegate Custom|TrySpawnClass) (Variables|Default|GetSpawnInterval) true))

(fn ConstructionScript)