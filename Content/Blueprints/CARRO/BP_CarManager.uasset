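; BP_CarManager is a traffic spawner that periodically creates BP_Car actors on splines.
; A looping timer started on BeginPlay picks a random CarSpline entry, gets its spline through GetSplineMessage, and spawns a car at the first point with that spline as ActiveSpline.
; An invalid spline triggers an immediate recursive retry.
; ActiveCars only counts spawns: upon reaching MaxCars, the next tick skips spawning and resets it to zero.
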(event Custom|TrySpawnClass
  (bind _carspline (Variables|Default|GetCarSpline))
  (if (< (Variables|Default|GetActiveCars) (Variables|Default|GetMaxCars))
    (bind _newparam (Class|BPIGetSpline|GetSpline(Message) (Utilities|Array|Get(acopy) _carspline (Math|Random|RandomIntegerinRange 0 (- (Utilities|Array|Length _carspline) 1)))))
    (bind _output_get (Variables|Default|SetNew%20Param _newparam))
    (Utilities|IsValid _output_get
      (:Is%20Valid
        (Game|SpawnActorfromClass "/Game/Blueprints/CARRO/BP_Car.BP_Car_C" (Math|Conversions|ToTransform(Vector) (Spline|GetLocationatSplinePoint _output_get 0 "World")) "Undefined" "MultiplyWithRoot" 0 _output_get 0)
        (Math|Integer|IncrementInt (Variables|Default|GetActiveCars)))
      (:Is%20Not%20Valid
        (CallFunction|TrySpawnClass)))
    (else
      (Variables|Default|SetActiveCars 0))))

(event EventBeginPlay
  (Utilities|Time|SetTimerbyEvent (delegate Custom|TrySpawnClass) (Variables|Default|GetSpawnInterval) true))

(fn ConstructionScript)