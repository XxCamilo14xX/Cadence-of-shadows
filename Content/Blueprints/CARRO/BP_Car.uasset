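; BP_Car is a car actor that advances along ActiveSpline every tick, matching its location and rotation to the spline.
; Traffic-light changes set TrafficState, but the switch mapping that state to Speed is disconnected, so the state never affects movement.
; At higher speeds, a FarDetection overlap sends a damage message to OverlappedComponent.
; The end-of-spline check leads nowhere, and DestroyActor is unwired.
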(event OnComponentBeginOverlap(FarDetection)
  (params (OverlappedComponent :type Primitive%20Component%20Object%20Reference) (OtherActor :type Actor%20Object%20Reference) (OtherComp :type Primitive%20Component%20Object%20Reference) (OtherBodyIndex :type Integer) (bFromSweep :type Boolean) (SweepResult :type Hit%20Result%20Structure%20%28by%20ref%29))
  (if (> (Variables|Default|GetSpeed) 1e+02)
    (Class|BPIDamagable|TakeDamage(Message) OverlappedComponent (Utilities|Struct|MakeS_DamageInfo 1e+01 "NewEnumerator4" "NewEnumerator3" false false false false))))

(event EventOnTrafficStateChanged
  (params (NewState :type E_TrafficState%20Enum :default "NewEnumerator0"))
  (switch Utilities|FlowControl|Switch|SwitchonE_TrafficState NewState
    (:NewEnumerator0
      (Variables|Default|SetTrafficState "NewEnumerator0"))
    (:NewEnumerator1
      (Variables|Default|SetTrafficState "NewEnumerator1"))
    (:NewEnumerator2
      (Variables|Default|SetTrafficState "NewEnumerator2"))))

(event EventTick
  (params (DeltaSeconds :type Float%20%28single-precision%29))
  (bind _activespline (Variables|Default|GetActiveSpline))
  (bind _output_get (Variables|Default|SetCurrentDistance (+ (Variables|Default|GetCurrentDistance) (* (Variables|Default|GetSpeed) (Utilities|Time|GetWorldDeltaSeconds)))))
  (Transformation|SetActorLocationAndRotation (Spline|GetLocationatDistanceAlongSpline _activespline _output_get "World") (Spline|GetRotationatDistanceAlongSpline _activespline _output_get "World"))
  (if (> (Spline|GetSplineLength _activespline) _output_get)
    _))

(fn ConstructionScript)