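; BPA_Recording is an inventory actor that stages an item's mesh in front of a SceneCaptureComponent2D, apparently to render an item preview.
; ClickInteract shows the mesh of the inventory item at the given index.
; UpdateStaticMesh swaps in a supplied mesh, moves the capture to its camera position and stores its min/max position limits, while ResetMesh clears it.
; AddItem, SubstractItem and InsViewing are stubs returning false.
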(event EventBeginPlay)

(event EventClickInteract
  (params (Index :type Integer))
  (Components|StaticMesh|SetStaticMesh (Variables|Default|GetStaticMesh) (.Mesh (Utilities|Struct|BreakS_ItemStruct (Utilities|Array|Get(acopy) (Variables|/Game/Blueprints/Components/BPC_Inventory.BPC_Inventory_C|GetItems (Variables|Default|GetBPC_Inventory)) Index)))))

(fn ConstructionScript)

(fn UpdateStaticMesh
  (params (NewMesh :type S%20Recording%20Item%20Settings%20Structure))
  (bind (_mesh _cameraposition _maxposition _minposition) (Utilities|Struct|BreakS_RecordingItemSettings NewMesh))
  (if (!= _mesh 0)
    (Components|StaticMesh|SetStaticMesh (Variables|Default|GetStaticMesh) _mesh)
    (Transformation|SetRelativeLocation (Variables|Default|GetSceneCaptureComponent2D) _cameraposition false false)
    (CallFunction|UpdatePosition _maxposition _minposition)))

(fn UpdatePosition
  (params (MaxPosition :type Float%20%28double-precision%29) (MinPosition :type Float%20%28double-precision%29))
  (Variables|Default|SetMinPosition MinPosition)
  (Variables|Default|SetMaxPosition MaxPosition))

(fn ResetMesh
  (Components|StaticMesh|SetStaticMesh (Variables|Default|GetStaticMesh) 0))

(fn AddItem
  (params (Item :type S%20Item%20Struct%20Structure))
  (return false))

(fn InsViewing
  (return false))

(fn SubstractItem
  (params (Item :type S%20Item%20Struct%20Structure) (Index :type Integer))
  (return false))