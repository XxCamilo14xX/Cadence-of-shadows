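; TP is an interactable fast-travel point that opens the travel map when a player interacts with it.
; On BeginPlay it passes its TeleportPoints to the BPCFasTravelManager component, and Interacti calls ShowMap on that manager.
; The interaction interface getters return default values for AP count, hold duration, location and interaction type.
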(event EventBeginPlay
  (Variables|/Game/FasTravel/BPC_FasTravelManager.BPC_FasTravelManager_C|SetTeleportPoints (Variables|Default|GetBPC_FasTravelManager) (Variables|Default|GetTeleport%20Points)))

(event EventInteracti
  (params (Interactor :type Actor%20Object%20Reference))
  (Default|ShowMap (Variables|Default|GetBPC_FasTravelManager)))

(fn ConstructionScript)

(fn GetApCount
  (return 0))

(fn GetHoldDuration
  (return 0.0))

(fn GetInteractionLocation
  (return "0, 0, 0"))

(fn GetTypeInteraction
  (return "NewEnumerator0"))