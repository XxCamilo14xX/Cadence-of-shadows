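; BP_Lamp3 is a lamp for the NorthBuildings map that switches its point light according to the time of day.
; Every Tick it looks up the SunMoonDaySequenceActor and reads its time of day.
; At or after OnTime it sets full intensity; otherwise, at or after OffTime it sets zero.
; Times earlier than both thresholds leave the light unchanged.
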(event EventTick
  (params (DeltaSeconds :type Float%20%28single-precision%29))
  (bind _returnvalue (Actor|GetActorOfClass "/Script/DaySequence.SunMoonDaySequenceActor"))
  (if (>= (Class|DaySequenceActor|GetTimeOfDay _returnvalue) (Variables|Default|GetOnTime))
    (Rendering|Components|Light|SetIntensity (Variables|Default|GetPointLight) 5e+03)
    (elif (>= (Class|DaySequenceActor|GetTimeOfDay _returnvalue) (Variables|Default|GetOffTime))
      (Rendering|Components|Light|SetIntensity (Variables|Default|GetPointLight) 0.0))))

(fn ConstructionScript)