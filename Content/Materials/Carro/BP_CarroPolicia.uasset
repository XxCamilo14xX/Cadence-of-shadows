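; BP_CarroPolicia is a police car Blueprint that alternates red and blue flashing lights.
; On BeginPlay it turns both lights off and starts a looping one-second timer bound to the cambiolucecitas event.
; Each tick of that timer checks and flips the Isred flag, setting one light to high intensity and the other to zero.
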(event Custom|cambiolucecitas
  (if (Variables|Default|GetIsred)
    (Rendering|Components|Light|SetIntensity (Variables|Default|GetBlue) 0.0)
    (Rendering|Components|Light|SetIntensity (Variables|Default|GetRed) 21006.316406)
    (Variables|Default|SetIsred false)
    (else
      (Rendering|Components|Light|SetIntensity (Variables|Default|GetBlue) 21006.316406)
      (Rendering|Components|Light|SetIntensity (Variables|Default|GetRed) 0.0)
      (Variables|Default|SetIsred true))))

(event EventBeginPlay
  (Rendering|Components|Light|SetIntensity (Variables|Default|GetBlue) 0.0)
  (Rendering|Components|Light|SetIntensity (Variables|Default|GetRed) 0.0)
  (Utilities|Time|SetTimerbyEvent (delegate Custom|cambiolucecitas) 1.0 true))

(fn ConstructionScript)