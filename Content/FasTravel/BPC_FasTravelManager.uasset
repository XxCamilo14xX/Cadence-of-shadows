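; Actor component that manages the fast travel menu widget and toggles it on screen.
; One second after BeginPlay it creates WB_FastMenu, stores it and passes itself to the widget's LoadFastTravel.
; ShowMap adds or removes the widget based on its visibility, switching the mouse cursor and input mode between game-and-UI and game-only.
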(event Custom|Show%20Map
  (bind _returnvalue (Game|GetPlayerController 0))
  (bind _returnvalue_2 (Game|GetPlayerController 0))
  (bind _widget (Variables|Default|GetWidget))
  (if (Widget|IsVisible (Variables|Default|GetWidget))
    (Widget|RemovefromParent _widget)
    (Variables|/Script/Engine.PlayerController|SetbShowMouseCursor _returnvalue false)
    (Input|SetInputModeGameOnly _returnvalue false)
    (else
      (Variables|/Script/Engine.PlayerController|SetbShowMouseCursor _returnvalue_2 true)
      (Input|SetInputModeGameandUI _returnvalue_2 0 "DoNotLock" true false)
      (UserInterface|Viewport|AddtoViewport _widget 0))))

(event EventBeginPlay
  (Utilities|FlowControl|Delay 1.0)
  (bind _returnvalue (UserInterface|CreateWidget "/Game/FasTravel/WB_FastMenu.WB_FastMenu_C"))
  (bind _output_get (Variables|Default|SetWidget _returnvalue))
  (Default|LoadFastTravel _output_get self))