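; Grunt enemy Blueprint that implements a short-range melee attack on top of parent enemy logic.
; Attack starts an end timer and, if not dead, sphere-traces forward for Pawns, ignoring all BP_Grunt actors.
; A hit sends blockable, parryable, interrupting damage via a TakeDamage message and signals attack end immediately.
; The timer also signals attack end, whether or not the trace hits.
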(event Custom|End%20Attack
  (Default|CallOnAttackEnd))

(event Custom|Attack
  (bind _returnvalue (Transformation|GetActorLocation))
  (Utilities|Time|SetTimerbyEvent (delegate Custom|End%20Attack) 0.5)
  (bind _outactors (Actor|GetAllActorsOfClass "/Game/Player_Enemies/Enemy/BP_Grunt.BP_Grunt_C"))
  (if (not (Variables|/Game/Blueprints/Components/BPC_DamgeSystem.BPC_DamgeSystem_C|GetIsDead (Variables|Default|GetBPC_DamgeSystem)))
    (bind (_outhit _returnvalue_2) (Collision|SphereTraceForObjects (+ _returnvalue (Math|Vector|MakeVector 0.0 0.0 3e+01)) (+ (+ _returnvalue (* (Transformation|GetActorForwardVector) 1.5e+02)) (Math|Vector|MakeVector 0.0 0.0 3e+01)) 2e+01 (Utilities|Array|MakeArray "ObjectTypeQuery3") false _outactors "ForOneFrame"))
    (if _returnvalue_2
      (Class|BPIDamagable|TakeDamage(Message) (.HitActor (Collision|BreakHitResult _outhit)) (Utilities|Struct|MakeS_DamageInfo (Variables|Default|GetAmount) (Variables|Default|GetDamage%20Type) "NewEnumerator1" false true true true))
      (Default|CallOnAttackEnd))))

(fn ConstructionScript
  (|CallParentFunction))