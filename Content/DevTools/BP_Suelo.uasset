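; BP_Suelo is a configurable floor actor in the DevTools folder, with an editable look and no active gameplay logic.
; The Construction Script assigns the chosen mesh and material to its StaticMesh component.
; It then pushes variables for two top colors, two side colors, tiling and roughness into the material parameters, so changes apply at construction.
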(event EventBeginPlay)

(event Collision|EventActorBeginOverlap
  (params (OtherActor :type Actor%20Object%20Reference)))

(event EventTick
  (params (DeltaSeconds :type Float%20%28single-precision%29)))

(fn ConstructionScript
  (Components|StaticMesh|SetStaticMesh (Variables|Default|GetStaticMesh) (Variables|Default|GetMesh))
  (Rendering|Material|SetMaterial (Variables|Default|GetStaticMesh) 0 (Variables|Default|GetMaterial))
  (Rendering|Material|SetVectorParameterValueonMaterials (Variables|Default|GetStaticMesh) "TopColor_1" (Math|Conversions|ToVector(LinearColor) (Variables|Default|GetTopColor%201)))
  (Rendering|Material|SetVectorParameterValueonMaterials (Variables|Default|GetStaticMesh) "TopColor_2" (Math|Conversions|ToVector(LinearColor) (Variables|Default|GetTopColor%202)))
  (Rendering|Material|SetVectorParameterValueonMaterials (Variables|Default|GetStaticMesh) "SideColor_1" (Math|Conversions|ToVector(LinearColor) (Variables|Default|GetSideColor%201)))
  (Rendering|Material|SetVectorParameterValueonMaterials (Variables|Default|GetStaticMesh) "SideColor_2" (Math|Conversions|ToVector(LinearColor) (Variables|Default|GetSideColor%202)))
  (Rendering|Material|SetScalarParameterValueonMaterials (Variables|Default|GetStaticMesh) "Tiling" (Variables|Default|GetTiling))
  (Rendering|Material|SetScalarParameterValueonMaterials (Variables|Default|GetStaticMesh) "Roughness" (Variables|Default|GetRoughness)))